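; BP_BasicEnemy is a basic enemy pawn that chases the first-person player character.
; On BeginPlay it runs parent init, caches its BP_BasicEnemyCont controller, gives that controller a back-reference, then caches player 0's character.
; While Enabled is true, Tick re-issues AI MoveTo toward the cached player every frame.
; An unconnected mesh-to-cube transform snap and a disabled overlap event are leftovers that never run.
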(event EventBeginPlay
  ;[0.15 0.15 0.15 0.5] Init Parent + Refs
  (|CallParentFunction)
  (bind _asbp_basic_enemy_cont (Utilities|Casting|CastToBP_BasicEnemyCont (Pawn|GetController)))
  (bind _output_get (Variables|Default|SetControllerRef _asbp_basic_enemy_cont))
  (Variables|/Game/Enemies/BasicEnemy/BP_BasicEnemyCont.BP_BasicEnemyCont_C|SetAIRef _output_get self)
  (bind _asbp_first_person_character (Utilities|Casting|CastToBP_FirstPersonCharacter (Game|GetPlayerCharacter 0)))
  (Variables|Default|SetPlayerRef _asbp_first_person_character))

(event Collision|EventActorBeginOverlap
  (params (OtherActor :type Actor%20Object%20Reference))
  (|CallParentFunction OtherActor) ; This node is disabled and will not be called.\nDrag off pins to build functionality.
)

(event EventTick
  (params (DeltaSeconds :type Float%20%28single-precision%29))
  (|CallParentFunction DeltaSeconds)
  (if (Variables|Default|GetEnabled)
    (AI|AIMoveTo self "0, 0, 0" (Variables|Default|GetPlayerRef) 5.0 false)))

(fn ConstructionScript
  (|CallParentFunction))