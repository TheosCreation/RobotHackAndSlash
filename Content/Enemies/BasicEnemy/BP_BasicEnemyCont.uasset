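; AI controller for the basic enemy that runs its behavior tree and feeds it blackboard data about the player.
; BeginPlay finds the first-person character, stores it as the target and enables movement, attack and active flags.
; Tick compares only X and Z positions against TrackingDistance, updating the target and location in range or disabling movement otherwise.
; ResetAttack re-enables attacking after a fixed delay, with a DoOnce blocking overlapping calls.
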(event Custom|ResetAttack
  ;[0.15 0.15 0.15 0.5] Reset Attack
  (Utilities|FlowControl|DoOnce false :!label _label
    (:Completed
      (Utilities|FlowControl|Delay 2.5)
      (AI|Components|Blackboard|SetValueasBool (Variables|Default|GetBlackboardRef) (Utilities|Name|MakeLiteralName "CanAttack") true)
      (goto _label Reset))))

(event EventBeginPlay
  ;[0.15 0.15 0.15 0.5] Init
  (AI|RunBehaviorTree "/Game/Enemies/BasicEnemy/BT_BasicEnemy.BT_BasicEnemy")
  (bind _returnvalue (Actor|GetActorOfClass "/Game/FirstPerson/Blueprints/BP_FirstPersonCharacter.BP_FirstPersonCharacter_C"))
  (bind _output_get (Variables|Default|SetPlayerRef _returnvalue))
  (AI|Components|Blackboard|SetValueasObject (Variables|Default|GetBlackboardRef) (Utilities|Name|MakeLiteralName "TargetActor") _output_get)
  (AI|Components|Blackboard|SetValueasBool (Variables|Default|GetBlackboardRef) (Utilities|Name|MakeLiteralName "CanMove") true)
  (AI|Components|Blackboard|SetValueasBool (Variables|Default|GetBlackboardRef) (Utilities|Name|MakeLiteralName "CanAttack") true)
  (AI|Components|Blackboard|SetValueasBool (Variables|Default|GetBlackboardRef) (Utilities|Name|MakeLiteralName "IsEnabled") true))

(event EventTick
  (params (DeltaSeconds :type Float%20%28single-precision%29))
  (bind _returnvalue (Utilities|Name|MakeLiteralName "CanMove"))
  (bind _playerref (Variables|Default|GetPlayerRef))
  (bind _blackboardref (Variables|Default|GetBlackboardRef))
  (bind _playerref_2 (Variables|Default|GetPlayerRef))
  (bind _airef (Variables|Default|GetAIRef))
  (bind _returnvalue_2 (Transformation|GetActorLocation _playerref))
  (bind _returnvalue_3 (Transformation|GetActorLocation _airef))
  ;[0.15 0.15 0.15 0.5] Update
  (if (<= (Math|Vector|Distance(Vector) (Math|Vector|MakeVector (.x _returnvalue_3) 0.0 (.z _returnvalue_3)) (Math|Vector|MakeVector (.x _returnvalue_2) 0.0 (.z _returnvalue_2))) (Variables|Default|GetTrackingDistance))
    (AI|Components|Blackboard|SetValueasVector (Variables|Default|GetBlackboardRef) (Utilities|Name|MakeLiteralName "TargetLocation") (Transformation|GetActorLocation _playerref_2))
    (AI|Components|Blackboard|SetValueasBool _blackboardref _returnvalue true)
    (AI|Components|Blackboard|SetValueasObject (Variables|Default|GetBlackboardRef) (Utilities|Name|MakeLiteralName "TargetActor") _playerref_2)
    (else
      (AI|Components|Blackboard|SetValueasBool _blackboardref _returnvalue false))))

(fn ConstructionScript)